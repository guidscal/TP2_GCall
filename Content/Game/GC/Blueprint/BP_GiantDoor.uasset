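; BP_GiantDoor is a giant two-part door made of mossy wall meshes that slide apart when opened.
; On BeginPlay it binds OpenDoor to an OpenGiantDoor event.
; OpenDoor plays a door sound at the root component's relative location and runs a timeline whose Ouverture track lerps both walls' relative X positions in opposite directions.
; The file contains no closing logic.
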(event `self.ReceiveBeginPlay`
  (add `self.OpenGiantDoor` (delegate `OpenDoor`)))

(event `OpenDoor`
  (`GameplayStatics.PlaySoundAtLocation` "/Game/Game/GC/Audio/S_PorteGeante_Cue.S_PorteGeante_Cue" (`SceneComponent.RelativeLocation` (`self.DefaultSceneRoot`)) (struct) 1.0 1.0 0.0 null null null null)
  (bind (_direction _ouverture) (`Timeline|Timeline`)
    (:`Update`
      (`SceneComponent.K2_SetRelativeLocation` (`self.MossyForgotten_Wall1`) (`KismetMathLibrary.MakeVector` (`KismetMathLibrary.Lerp` 1180.0 1500.0 _ouverture)) false false)
      (`SceneComponent.K2_SetRelativeLocation` (`self.MossyForgotten_Wall`) (`KismetMathLibrary.MakeVector` (`KismetMathLibrary.Lerp` 0.0 -320.0 _ouverture)) false false))))

(fn `UserConstructionScript`)