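; Actor that periodically spawns BP_Bomb at its own transform while the player character is inside its Box trigger.
; BeginPlay waits a random delay up to FrequenceBombes, then starts a looping timer at that interval, so the first drop varies per spawner.
; Box overlap events with BP_ThirdPersonCharacter toggle IsPlayerOverlapping, which each timer tick checks before spawning.
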(event `self.ReceiveBeginPlay`
  ; Randomise le temps avant la premiere bombe
  (`KismetSystemLibrary.Delay` (`KismetMathLibrary.RandomFloatInRange` 0.0 (`self.FrequenceBombes`)))
  (`KismetSystemLibrary.K2_SetTimerDelegate` (delegate `SpawnBomb`) (`self.FrequenceBombes`) true))

(event `SpawnBomb`
  (if (`self.IsPlayerOverlapping`)
    (`|SpawnActorFromClass` "/Game/Game/Blueprints/Actors/BP_Bomb.BP_Bomb_C" (`self.GetTransform`) "Undefined" "MultiplyWithRoot" null null)))

(event `self.Box.OnComponentBeginOverlap`
  (params (OverlappedComponent :type "PrimitiveComponent Object Reference") (OtherActor :type "Actor Object Reference") (OtherComp :type "PrimitiveComponent Object Reference") (OtherBodyIndex :type Integer) (bFromSweep :type Boolean) (SweepResult :type "HitResult Structure (by ref)"))
  (cast `/Game/Game/Blueprints/Pawns_Characters/Player/BP_ThirdPersonCharacter` OtherActor)
  (set `self.IsPlayerOverlapping` true))

(event `self.Box.OnComponentEndOverlap`
  (params (OverlappedComponent :type "PrimitiveComponent Object Reference") (OtherActor :type "Actor Object Reference") (OtherComp :type "PrimitiveComponent Object Reference") (OtherBodyIndex :type Integer))
  (cast `/Game/Game/Blueprints/Pawns_Characters/Player/BP_ThirdPersonCharacter` OtherActor)
  (set `self.IsPlayerOverlapping` false))

(fn `UserConstructionScript`)