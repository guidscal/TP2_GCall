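; BP_Plateform is a crumbling wooden platform that breaks after being triggered and respawns later.
; An overlap on its Box starts a one-shot sequence guarded by an Active flag, playing a creaking-break sound, then a final break sound after a delay.
; The WeightedWoodPlatform mesh is then hidden with collision disabled until a second delay restores it and rearms the trigger.
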(event `self.Box.OnComponentBeginOverlap`
  (params (OverlappedComponent :type "PrimitiveComponent Object Reference") (OtherActor :type "Actor Object Reference") (OtherComp :type "PrimitiveComponent Object Reference") (OtherBodyIndex :type Integer) (bFromSweep :type Boolean) (SweepResult :type "HitResult Structure (by ref)"))
  (if (not (`self.bActive`))
    (set `self.bActive` true)
    (`GameplayStatics.PlaySound2D` "/Game/Game/Audio/SFX/S_WoodBreaking.S_WoodBreaking" 1.0 1.0 0.0 null null)
    (`KismetSystemLibrary.Delay` 3.0)
    (`GameplayStatics.PlaySound2D` "/Game/Game/Audio/SFX/S_WoodBreak.S_WoodBreak" 1.0 1.0 0.0 null null)
    (`SceneComponent.SetVisibility` (`self.Weighted_Wood_Platform`) false false)
    (`PrimitiveComponent.SetCollisionEnabled` (`self.Weighted_Wood_Platform`) "NoCollision")
    (`KismetSystemLibrary.Delay` 5.0)
    (`SceneComponent.SetVisibility` (`self.Weighted_Wood_Platform`) true false)
    (`PrimitiveComponent.SetCollisionEnabled` (`self.Weighted_Wood_Platform`) "QueryAndPhysics")
    (`PrimitiveComponent.SetCollisionEnabled` (`self.Box`) "QueryOnly")
    (set `self.bActive` false)))

(fn `UserConstructionScript`)