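; Player state Blueprint that persists the player's health through the game instance and triggers respawn on death.
; On BeginPlay it restores saved health into its health component, or resets health and marks it initialized on first run.
; Health changes are written back to the game instance, and death asks the third-person game mode to start respawning player controller 0.
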(event `self.ReceiveBeginPlay`
  (bind _asbp_game_instance (cast `/Game/Game/Blueprints/GameInstance/BP_GameInstance` (`GameplayStatics.GetGameInstance`)))
  (bind _output_get (set `self.RefGameInstance` _asbp_game_instance))
  (if (`/Game/Game/Blueprints/GameInstance/BP_GameInstance.HealthInitialize_GI` _output_get)
    (`self.LoadHealthFromGameInstance`)
    (else
      (`/Game/Game/Blueprints/Components/AC_Health.ResetHealth` (`self.AC_Health`))
      (set `/Game/Game/Blueprints/GameInstance/BP_GameInstance.HealthInitialize_GI` true (`self.RefGameInstance`)))))

(event `self.AC_Health.OnDeath`
  (bind _asbp_third_person_game_mode (cast `/Game/Game/Blueprints/GameMode/BP_ThirdPersonGameMode` (`GameplayStatics.GetGameMode`)))
  (`/Game/Game/Blueprints/GameMode/BP_ThirdPersonGameMode.StartRespawn` _asbp_third_person_game_mode (`GameplayStatics.GetPlayerController` 0)))

(event `self.AC_Health.OnHealthChanged`
  (params (CurrentHealth :type "Float (double-precision)") (MaxHealth :type "Float (double-precision)"))
  (`self.SaveCurrentHealth` CurrentHealth)
  (`self.SaveMaxHealth` MaxHealth))

(fn `LoadHealthFromGameInstance`
  (bind _output_get (set `/Game/Game/Blueprints/Components/AC_Health.MaxHealth` (`/Game/Game/Blueprints/GameInstance/BP_GameInstance.MaxHealth_GI` (`self.RefGameInstance`)) (`self.AC_Health`)))
  (bind _output_get_2 (set `/Game/Game/Blueprints/Components/AC_Health.CurrentHealth` (`/Game/Game/Blueprints/GameInstance/BP_GameInstance.CurrentHealth_GI` (`self.RefGameInstance`)) (`self.AC_Health`)))
  (`/Game/Game/Blueprints/Components/AC_Health.OnHealthChanged` (`self.AC_Health`) _output_get_2 _output_get))

(fn `SaveCurrentHealth`
  (params (NewHealth :type "Float (double-precision)"))
  (set `/Game/Game/Blueprints/GameInstance/BP_GameInstance.CurrentHealth_GI` NewHealth (`self.RefGameInstance`)))

(fn `SaveMaxHealth`
  (params (NewMaxHealth :type "Float (double-precision)"))
  (set `/Game/Game/Blueprints/GameInstance/BP_GameInstance.MaxHealth_GI` NewMaxHealth (`self.RefGameInstance`)))

(fn `UserConstructionScript`)