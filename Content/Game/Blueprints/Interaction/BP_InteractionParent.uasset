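; BP_InteractionParent is a base interactable actor that can act as a points pickup or a giant-door opener.
; The construction script configures its mesh, sphere trigger and prompt widget from variables.
; Trigger overlaps register or unregister it with BP_ThirdPersonCharacter, and ToggleUI controls prompt visibility.
; Interact either awards points through BPI_PointManager with a sound, or pulls all levers and opens all giant doors, destroying itself in both cases.
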(event `self.InteractTrigger.OnComponentBeginOverlap`
  (params (OverlappedComponent :type "PrimitiveComponent Object Reference") (OtherActor :type "Actor Object Reference") (OtherComp :type "PrimitiveComponent Object Reference") (OtherBodyIndex :type Integer) (bFromSweep :type Boolean) (SweepResult :type "HitResult Structure (by ref)"))
  (bind _asbp_third_person_character (cast `/Game/Game/Blueprints/Pawns_Characters/Player/BP_ThirdPersonCharacter` OtherActor))
  (`/Game/Game/Blueprints/Pawns_Characters/Player/BP_ThirdPersonCharacter.AddInteraction` _asbp_third_person_character self))

(event `self.InteractTrigger.OnComponentEndOverlap`
  (params (OverlappedComponent :type "PrimitiveComponent Object Reference") (OtherActor :type "Actor Object Reference") (OtherComp :type "PrimitiveComponent Object Reference") (OtherBodyIndex :type Integer))
  (bind _asbp_third_person_character (cast `/Game/Game/Blueprints/Pawns_Characters/Player/BP_ThirdPersonCharacter` OtherActor))
  (`/Game/Game/Blueprints/Pawns_Characters/Player/BP_ThirdPersonCharacter.RemoveInteraction` _asbp_third_person_character self))

(fn `Interact`
  (params (Character :type "/Game/Game/Blueprints/Pawns_Characters/Player/BP_ThirdPersonCharacter Object Reference"))
  (bind _output_get (set `self.InteractCharacter` Character))
  (`|ExecutionSequence`
    (:`then_0`
      (if (`self.Is Points Item`)
        (if (`KismetSystemLibrary.DoesImplementInterface` _output_get "/Game/Game/Blueprints/Interfaces/BPI_PointManager.BPI_PointManager_C")
          (message `/Game/Game/Blueprints/Interfaces/BPI_PointManager.AddPoints` _output_get (`self.GainPoints`))
          (`GameplayStatics.PlaySound2D` "/Game/Game/Audio/SFX/Money.Money" 1.0 1.0 0.0 null null)
          (`self.K2_DestroyActor`))))
    (:`then_1`
      (if (`self.IsDoorOpener`)
        (bind _outactors (`GameplayStatics.GetAllActorsOfClass` "/Game/Game/GC/Blueprint/BP_LevierPorteGeante.BP_LevierPorteGeante_C"))
        (for _array_element _outactors
          (`/Game/Game/GC/Blueprint/BP_LevierPorteGeante.Pull Lever` _array_element)
          (bind _outactors_2 (`GameplayStatics.GetAllActorsOfClass` "/Game/Game/GC/Blueprint/BP_GiantDoor.BP_GiantDoor_C"))
          (for _array_element_2 _outactors_2
            (`/Game/Game/GC/Blueprint/BP_GiantDoor.OpenDoor` _array_element_2)
            (`self.K2_DestroyActor`)))))))

(fn `SetupMesh`
  ; Setup Mesh type and location
  (`StaticMeshComponent.SetStaticMesh` (`self.InteractMesh`) (`self.InteractionMesh`))
  (`SceneComponent.K2_SetRelativeTransform` (`self.InteractMesh`) (`self.MeshTransform`) false false))

(fn `SetupTrigger`
  ; Setup trigger area
  (`SphereComponent.SetSphereRadius` (`self.InteractTrigger`) (`self.TriggerRadius`) true)
  (`SceneComponent.K2_SetRelativeLocation` (`self.InteractTrigger`) (`self.TriggerLocation`) false false))

(fn `SetupUI`
  ; Setup UI and set offset
  (`SceneComponent.K2_SetRelativeLocation` (`self.InteractUI`) (`self.UILocation`) false false))

(fn `ToggleUI`
  (params (isVisible :type Boolean))
  ; Add interact prompt to screen
  (`SceneComponent.SetVisibility` (`self.InteractUI`) isVisible false))

(fn `UserConstructionScript`
  ; Construct
  (`self.SetupMesh`)
  (`self.SetupTrigger`)
  (`self.SetupUI`))